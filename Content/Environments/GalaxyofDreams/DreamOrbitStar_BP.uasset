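; DreamOrbitStar_BP is a Galaxy of Dreams environment actor that continuously spins its static mesh about the vertical axis.
; BeginPlay picks a random signed yaw step, re-rolling whenever the value is near zero so every instance visibly turns in either direction.
; Tick adds that step to the mesh's world yaw each frame without delta-time scaling, so spin speed depends on frame rate.
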(event `self.ReceiveBeginPlay`
  (bind _output_get (set `self.Rotate` (`KismetMathLibrary.RandomFloatInRange` -3.0 3.0) :!label _label))
  (if (`KismetMathLibrary.InRange_FloatFloat` _output_get -0.49 0.49)
    (goto _label)))

(event `self.ReceiveTick`
  (params (DeltaSeconds :type "Float (single-precision)"))
  (bind _staticmesh (`self.StaticMesh`))
  (`SceneComponent.K2_SetWorldRotation` _staticmesh (`KismetMathLibrary.MakeRotator` (.roll (`SceneComponent.K2_GetComponentRotation` _staticmesh)) (.pitch (`SceneComponent.K2_GetComponentRotation` _staticmesh)) (+ (.yaw (`SceneComponent.K2_GetComponentRotation` _staticmesh)) (`self.Rotate`))) false false))

(fn `UserConstructionScript`)