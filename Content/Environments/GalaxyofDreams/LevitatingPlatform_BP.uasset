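; Levitating platform for the Galaxy of Dreams environment that moves back and forth between its start and an End component's position.
; On BeginPlay a timeline lerps between the two captured world locations, applying the result as the platform's relative location.
; When the timeline finishes it reverses, then plays forward again after a delay.
; An alternative sine-wave bobbing setup is left disconnected and never runs.
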(event `self.ReceiveTick`
  (params (DeltaSeconds :type "Float (single-precision)"))
  ;[1 1 1] Floating
)

(event `self.ReceiveBeginPlay`
  (set `self.StartLoc` (`SceneComponent.K2_GetComponentLocation` (`self.DreamPlatform`)))
  (set `self.EndLoc` (`SceneComponent.K2_GetComponentLocation` (`self.End`)))
  (bind (_direction _newtrack_0) (`Timeline|Forward Timeline` :!label _label)
    (:`Update`
      (`SceneComponent.K2_SetRelativeLocation` (`self.DreamPlatform`) (`KismetMathLibrary.VLerp` (`self.StartLoc`) (`self.EndLoc`) _newtrack_0) false false)
      (`KismetSystemLibrary.Delay` 5.0))
    (:`Finished`
      (`self.Down`) ; Finished plays after Update
      (`KismetSystemLibrary.Delay` 7.0)
      (`self.StartMove`))))

(event `StartMove`
  (goto _label))

(event `Down`
  (goto _label :!via `Reverse`))

(fn `UserConstructionScript`)