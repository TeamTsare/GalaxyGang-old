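; DreamGate_BP is a double gate in the Galaxy of Dreams environment that swings open when the player character's OpenTest flag is set.
; Every Tick it casts the player character to CharacterDanny and reads that flag, which comments tie to pressing E.
; While the flag is true it plays left and right timelines, whose DoorRot outputs set the relative yaw of the Left and Right components.
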(event `self.ReceiveTick`
  (params (DeltaSeconds :type "Float (single-precision)"))
  (bind _ascharacter_danny (cast `/Game/Characters/Char_Danny/CharacterDanny` (`GameplayStatics.GetPlayerCharacter` 0)))
  (if (`/Game/Characters/Char_Danny/CharacterDanny.OpenTest` _ascharacter_danny)
    (`|ExecutionSequence`
      (:`then_0`
        (bind (_direction _doorrot) (`Timeline|LeftTimeline`) ; When E is pressed time Timeline will play
          (:`Update`
            (`SceneComponent.K2_SetRelativeRotation` (`self.Left`) (`KismetMathLibrary.MakeRotator` 0.0 0.0 _doorrot) false false))))
      (:`then_1`
        (bind (_direction_2 _doorrot_2) (`Timeline|RightTimeline`) ; When E is pressed time Timeline will play
          (:`Update`
            (`SceneComponent.K2_SetRelativeRotation` (`self.Right`) (`KismetMathLibrary.MakeRotator` 0.0 0.0 _doorrot_2) false false)))))))

(fn `UserConstructionScript`)