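; CannonHatch1_BP is a Pirate Planet cannon hatch whose Door component is meant to swing on a sine wave.
; BeginPlay stores the X of the door's world forward vector as an offset.
; Tick rebuilds world rotation from that vector, replacing X with amplitude times sine plus offset and keeping Y and Z.
; The sine input multiplies time by zero, so as written the oscillation stays at zero.
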(event `self.ReceiveTick`
  (params (DeltaSeconds :type "Float (single-precision)"))
  (`SceneComponent.K2_SetWorldRotation` (`self.Door`) (`KismetMathLibrary.Conv_VectorToRotator` (`KismetMathLibrary.MakeVector` (+ (* (`self.RotAmp`) (`KismetMathLibrary.DegSin` (* (`self.RotFreq`) 0.0 (`GameplayStatics.GetTimeSeconds`)))) (`self.RotOffset`)) (.y (`KismetMathLibrary.Conv_RotatorToVector` (`SceneComponent.K2_GetComponentRotation` (`self.Door`)))) (.z (`KismetMathLibrary.Conv_RotatorToVector` (`SceneComponent.K2_GetComponentRotation` (`self.Door`)))))) false false))

(event `self.ReceiveBeginPlay`
  (set `self.RotOffset` (.x (`KismetMathLibrary.Conv_RotatorToVector` (`SceneComponent.K2_GetComponentRotation` (`self.Door`))))))

(fn `UserConstructionScript`)