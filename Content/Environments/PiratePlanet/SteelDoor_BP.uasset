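; Pirate planet steel door that opens when the player character's OpenTest flag is set.
; Tick polls the flag on CharacterDanny, then plays a timeline that lerps the Door from its start to the End component's location, both cached at BeginPlay in world space but applied as relative location.
; The Wheel rotates every tick while the flag holds; the delayed zero rotation does not stop it.
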(event `self.ReceiveBeginPlay`
  (set `self.StartLoc` (`SceneComponent.K2_GetComponentLocation` (`self.Door`)))
  (set `self.EndLoc` (`SceneComponent.K2_GetComponentLocation` (`self.End`))))

(event `self.ReceiveTick`
  (params (DeltaSeconds :type "Float (single-precision)"))
  (bind _ascharacter_danny (cast `/Game/Characters/Char_Danny/CharacterDanny` (`GameplayStatics.GetPlayerCharacter` 0)))
  (if (`/Game/Characters/Char_Danny/CharacterDanny.OpenTest` _ascharacter_danny)
    (`|ExecutionSequence`
      (:`then_0`
        (bind (_direction _newtrack_0) (`Timeline|Timeline_0`)
          (:`Update`
            (`SceneComponent.K2_SetRelativeLocation` (`self.Door`) (`KismetMathLibrary.VLerp` (`self.StartLoc`) (`self.EndLoc`) _newtrack_0) false false))))
      (:`then_1`
        (`SceneComponent.K2_AddLocalRotation` (`self.Wheel`) (struct :`Pitch` -10.0) false false)
        (`KismetSystemLibrary.Delay` 3.0)
        (`SceneComponent.K2_AddLocalRotation` :`self` (`self.Wheel`))))))

(fn `UserConstructionScript`)