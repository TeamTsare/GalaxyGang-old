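; Underwater steel door for the Pirate Planet environment, with two wheels that spin while two door meshes swing open.
; Tick polls the OpenTest flag on the player's CharacterDanny and clears it after a two-second delay.
; While the flag is set, both wheels rotate every frame and a timeline drives the yaw of both doors.
; The Blueprint itself makes no proximity check, relying entirely on that player flag.
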(event `self.ReceiveTick`
  (params (DeltaSeconds :type "Float (single-precision)"))
  (`|ExecutionSequence`
    (:`then_0`
      (bind _ascharacter_danny (cast `/Game/Characters/Char_Danny/CharacterDanny` (`GameplayStatics.GetPlayerCharacter` 0)))
      (if (`/Game/Characters/Char_Danny/CharacterDanny.OpenTest` _ascharacter_danny)
        (`KismetSystemLibrary.Delay` 2.0)
        (set `/Game/Characters/Char_Danny/CharacterDanny.OpenTest` false _ascharacter_danny)))
    (:`then_1`
      (if (`/Game/Characters/Char_Danny/CharacterDanny.OpenTest` _ascharacter_danny)
        (`SceneComponent.K2_AddLocalRotation` (`self.Wheel2`) (struct :`Pitch` -10.0) false false)
        (`SceneComponent.K2_AddLocalRotation` (`self.Wheel1`) (struct :`Pitch` -10.0) false false)
        (bind (_direction _doorrot) (`Timeline|Timeline_1`) ; When E is pressed time Timeline will play
          (:`Update`
            (`SceneComponent.K2_SetRelativeRotation` (`self.Door2`) (`KismetMathLibrary.MakeRotator` 0.0 0.0 _doorrot) false false)
            (`SceneComponent.K2_SetRelativeRotation` (`self.Door1`) (`KismetMathLibrary.MakeRotator` 0.0 0.0 _doorrot) false false)))
        (else
          (`SceneComponent.K2_AddLocalRotation` :`self` (`self.Wheel2`))
          (`SceneComponent.K2_AddLocalRotation` :`self` (`self.Wheel1`)))))))

(fn `UserConstructionScript`)