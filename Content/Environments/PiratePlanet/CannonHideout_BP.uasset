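; CannonHideout_BP is a Pirate Planet environment Blueprint that animates a pair of cannon hideout hatches.
; A timeline starts at BeginPlay and drives the roll of both hatches, which keep opposite fixed yaw angles.
; Its Finished output reverses it, then replays it after a delay, cycling the hatches without player input.
; Tick checks the Danny character's OpenTest flag but acts on neither result.
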(event `self.ReceiveBeginPlay`
  (bind (_direction _doorrot) (`Timeline|Timeline_0` :!label _label) ; When E is pressed time Timeline will play
    (:`Update`
      (`SceneComponent.K2_SetRelativeRotation` (`self.Hatch1`) (`KismetMathLibrary.MakeRotator` _doorrot 0.0 -11.0) false false)
      (`SceneComponent.K2_SetRelativeRotation` (`self.Hatch2`) (`KismetMathLibrary.MakeRotator` _doorrot 0.0 11.0) false false)
      (`KismetSystemLibrary.Delay` 2.0))
    (:`Finished`
      (`self.End`)
      (`KismetSystemLibrary.Delay` 2.0)
      (`self.Start`))))

(event `Start`
  (goto _label))

(event `End`
  (goto _label :!via `Reverse`))

(event `self.ReceiveTick`
  (params (DeltaSeconds :type "Float (single-precision)"))
  (bind _ascharacter_danny (cast `/Game/Characters/Char_Danny/CharacterDanny` (`GameplayStatics.GetPlayerCharacter` 0)))
  (if (`/Game/Characters/Char_Danny/CharacterDanny.OpenTest` _ascharacter_danny)
    _))

(fn `UserConstructionScript`)