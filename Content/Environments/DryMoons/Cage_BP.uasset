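; Cage actor whose door opens when the player character's OpenTest flag is set, then closes again.
; Tick polls the flag on CharacterDanny and plays a timeline that lerps the door from its starting location to the End component's location.
; On finish, the timeline reverses, and after a short delay OpenTest is cleared.
; Locations are captured in world space but applied as relative locations.
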(event `self.ReceiveBeginPlay`
  (set `self.StartLoc` (`SceneComponent.K2_GetComponentLocation` (`self.Door`)))
  (set `self.EndLoc` (`SceneComponent.K2_GetComponentLocation` (`self.End`))))

(event `self.ReceiveTick`
  (params (DeltaSeconds :type "Float (single-precision)"))
  (bind _ascharacter_danny (cast `/Game/Characters/Char_Danny/CharacterDanny` (`GameplayStatics.GetPlayerCharacter` 0)))
  (if (`/Game/Characters/Char_Danny/CharacterDanny.OpenTest` _ascharacter_danny)
    (bind (_direction _newtrack_0) (`Timeline|Timeline_1` :!label _label)
      (:`Update`
        (`SceneComponent.K2_SetRelativeLocation` (`self.Door`) (`KismetMathLibrary.VLerp` (`self.StartLoc`) (`self.EndLoc`) _newtrack_0) false false)
        (`KismetSystemLibrary.Delay` 5.0))
      (:`Finished`
        (`self.Down`) ; Finished plays after Update
        (`KismetSystemLibrary.Delay` 1.0) ; This stops the OpenTest from being Set to False every frame
        (bind _ascharacter_danny_2 (cast `/Game/Characters/Char_Danny/CharacterDanny` (`GameplayStatics.GetPlayerCharacter` 0)))
        (set `/Game/Characters/Char_Danny/CharacterDanny.OpenTest` false _ascharacter_danny_2)
        (`KismetSystemLibrary.PrintString` "Closed")))))

(event `Down`
  (goto _label :!via `Reverse`))

(fn `UserConstructionScript`)